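; BP_Spider_01 is an enemy spider character that chases the player and plays an attack montage when close.
; BeginPlay starts an AI Move To on the player, repeating after a short delay only when the move succeeds.
; Tick checks distance against AttackRange and whether the montage is already playing, then deactivates character movement during the attack and reactivates it on montage completion.
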(event `self.ReceiveBeginPlay`
  (`|AIMoveTo` self (0.0 0.0 0.0) (`GameplayStatics.GetPlayerCharacter` 0) :!label _label
    (:`OnSuccess`
      (`KismetSystemLibrary.Delay` 0.2)
      (goto _label))))

(event `self.ReceiveTick`
  (params (DeltaSeconds :type "Float (single-precision)"))
  (if (and (`self.IsAttackRange`) (not (`self.IsAttacking`)))
    (`ActorComponent.Deactivate` (`self.CharacterMovement`))
    (`|PlayMontage` (`self.Mesh`) "/Game/Characters/Enemy_Great_Spider/Animations/AM_SpiderAttac.AM_SpiderAttac"
      (:`OnCompleted`
        (`ActorComponent.Activate` (`self.CharacterMovement`) false)))))

(fn `IsAttacking`
  (returns (ReturnValue :type Boolean))
  (return (`AnimInstance.Montage_IsPlaying` (`SkeletalMeshComponent.GetAnimInstance` (`self.Mesh`)) "/Game/Characters/Enemy_Great_Spider/Animations/AM_SpiderAttac.AM_SpiderAttac")))

(fn `IsAttackRange`
  (returns (ReturnValue :type Boolean))
  (return (< (`self.GetDistanceTo` (`GameplayStatics.GetPlayerCharacter` 0)) (`self.AttackRange`))))

(fn `UserConstructionScript`)