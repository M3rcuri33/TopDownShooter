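; Player character Blueprint that creates the player HUD, moves along its capsule's forward and right axes, and fires a weapon effect.
; Each tick, mouse velocity above a dead zone sets a yaw from its direction via Atan2, and control rotation interpolates toward it.
; Fire input toggles the assault rifle muzzle flash and firing sound, playing an end sound on release; no hit or damage logic is present.
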(event `self.ReceiveBeginPlay`
  ;[0.3757 0.6898 1] HUD
  (bind _returnvalue (`|CreateWidget` "/Game/UI/W_PlayerHUD_01.W_PlayerHUD_01_C" null self))
  (`UserWidget.AddToViewport` _returnvalue 0))

(event `self.ReceiveTick`
  (params (DeltaSeconds :type "Float (single-precision)"))
  (`self.Rotate Character`))

(event `InputAxis|MoveForwardBack`
  (params (AxisValue :type "Float (single-precision)"))
  ;[0.6248 0.3933 1] Movement
  (`self.AddMovementInput` (`SceneComponent.GetForwardVector` (`self.CapsuleComponent`)) AxisValue))

(event `InputAxis|MoveLeftRight`
  (params (AxisValue :type "Float (single-precision)"))
  ;[0.6248 0.3933 1] Movement
  (`self.AddMovementInput` (`SceneComponent.GetRightVector` (`self.CapsuleComponent`)) AxisValue))

(event `InputAction|Fire`
  (params (Key :type "Key Structure"))
  (bind _p_assaultrifle_mf (`self.P_AssaultRifle_MF`))
  ;[1 0.5505 0.9003] Weapon Fire
  (:`Pressed`
    (`ActorComponent.Activate` _p_assaultrifle_mf false)
    (bind _returnvalue (`GameplayStatics.SpawnSound2D` "/Game/Sounds/Weapon_AssaultRifle/Stereo/SC_WeaponFire.SC_WeaponFire" 1.0 1.0 0.0 null))
    (set `self.Weapon Sound` _returnvalue))
  (:`Released`
    (`ActorComponent.Deactivate` _p_assaultrifle_mf)
    (`AudioComponent.Stop` (`self.Weapon Sound`))
    (`GameplayStatics.SpawnSound2D` "/Game/Sounds/Weapon_AssaultRifle/Stereo/SC_WeaponFireEnd.SC_WeaponFireEnd" 1.0 1.0 0.0 null)))

(fn `IsMouseDeadZone`
  (returns (ReturnValue :type Boolean))
  (return (> (`KismetMathLibrary.VSize2D` (`self.MouseVelocity`)) (`self.DeadZone`))))

(fn `MouseVelocity`
  (returns (ReturnValue :type "Vector2D Structure"))
  (bind (_deltax _deltay) (`PlayerController.GetInputMouseDelta` (`GameplayStatics.GetPlayerController` 0)))
  (return (/ (`KismetMathLibrary.MakeVector2D` _deltax _deltay) (`GameplayStatics.GetWorldDeltaSeconds`))))

(fn `Rotate Character`
  (bind _returnvalue (`GameplayStatics.GetPlayerController` 0))
  (bind (_returnvalue_x _returnvalue_y) (`KismetMathLibrary.BreakVector2D` (`self.MouseVelocity`)))
  (if (`self.IsMouseDeadZone`)
    (`Controller.SetControlRotation` _returnvalue (`KismetMathLibrary.RInterpTo` (`Controller.GetControlRotation` _returnvalue) (`KismetMathLibrary.MakeRotator` 0.0 0.0 (`KismetMathLibrary.DegAtan2` _returnvalue_x _returnvalue_y)) (`GameplayStatics.GetWorldDeltaSeconds`) (`self.Interp Speed`)))))

(fn `UserConstructionScript`)